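; Player controller for the SoloTask map that manages the start menu, player readiness and camera switching.
; After a short delay on BeginPlay it opens the menu through BP_SoloTask_HUD and caches all camera actors.
; Menu events toggle pawn input, while ready events pass state to the GameMode and refresh the menu widget.
; Other events set the pawn's transform and cycle blended view targets through the cameras.
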(event Custom|Close%20StartMenu
  (bind _returnvalue (Pawn|GetControlledPawn))
  (bind _asbp_solo_task_hud (Utilities|Casting|CastToBP_SoloTask_HUD (HUD|GetHUD)))
  (Default|DeleteStartMenu _asbp_solo_task_hud)
  ;[1 1 1] Must be false
  (Variables|Default|SetbShowMouseCursor true)
  (Utilities|IsValid _returnvalue
    (:Is%20Valid
      (Input|EnableInput _returnvalue self))
    (:Is%20Not%20Valid
      (Class|AutomationBlueprintFunctionLibrary|AddExpectedLogError "PlayerController: Controlled Pawn os not Valid"))))

(event Custom|Open%20StartMenu
  (bind _returnvalue (Pawn|GetControlledPawn))
  (bind _asbp_solo_task_hud (Utilities|Casting|CastToBP_SoloTask_HUD (HUD|GetHUD)))
  (Default|DrawStartMenu _asbp_solo_task_hud)
  (Variables|Default|SetbShowMouseCursor true)
  (Utilities|IsValid _returnvalue
    (:Is%20Valid
      (Input|DisableInput _returnvalue self))
    (:Is%20Not%20Valid
      (Class|AutomationBlueprintFunctionLibrary|AddExpectedLogError "PlayerController: Controlled Pawn os not Valid"))))

(event Custom|Server%20Update%20Player%20Ready
  (params (IsReady :type Boolean))
  (bind _asbp_solo_task_game_mode (Utilities|Casting|CastToBP_SoloTask_GameMode (Game|GetGameMode)))
  (Default|SetPlayerIsReady _asbp_solo_task_game_mode self IsReady))

(event Custom|Update%20Player%20Ready
  (bind _asbp_solo_task_hud (Utilities|Casting|CastToBP_SoloTask_HUD (HUD|GetHUD)))
  (Utilities|IsValid (Variables|/Game/Maps/SoloTask/WorldSettings/BP_SoloTask_HUD.BP_SoloTask_HUD_C|GetStart%20Menu _asbp_solo_task_hud)
    (:Is%20Valid
      (Default|UpdatePlayerReady (Variables|/Game/Maps/SoloTask/WorldSettings/BP_SoloTask_HUD.BP_SoloTask_HUD_C|GetStart%20Menu _asbp_solo_task_hud)))
    (:Is%20Not%20Valid
      (Class|AutomationBlueprintFunctionLibrary|AddExpectedLogError "PlayerController: Widget Start Menu is not Valid"))))

(event Custom|Change%20Camera
  (Game|Player|SetViewTargetwithBlend (Utilities|Array|Get(acopy) (Variables|Default|GetCameras) (Variables|Default|GetCurrentCamera)) 0.5 "VTBlend_Linear" 0.0 false)
  (Variables|Default|SetCurrentCamera (Math|Integer|%(Integer) (+ (Variables|Default|GetCurrentCamera) 1) (Utilities|Array|Length (Variables|Default|GetCameras)))))

(event Custom|Update%20Loc/Rot
  (params (Location :type Vector) (Rotation :type Rotator))
  (bind _returnvalue (Pawn|GetControlledPawn))
  (Transformation|SetActorLocation _returnvalue Location false false)
  (Transformation|SetActorRotation _returnvalue Rotation))

(event EventBeginPlay
  (Viewport|RemoveAllWidgets)
  (Utilities|FlowControl|Delay 0.5)
  (CallFunction|OpenStartMenu)
  (bind _outactors (Actor|GetAllActorsOfClass "/Script/Engine.CameraActor"))
  (Variables|Default|SetCameras _outactors))

(event Input|KeyboardEvents|P
  (params (Key :type Key%20Structure :default "None")))

(fn ConstructionScript)