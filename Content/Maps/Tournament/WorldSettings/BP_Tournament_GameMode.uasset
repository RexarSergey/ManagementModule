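; Tournament game mode that runs randomly paired knockout rounds of 1v1 arena matches until one player remains, then logs the win.
; CreateMatches splits logged-in players into two index-paired lists, has player controllers generate arenas, then teleports each pair to its arena's spawn points.
; UpdateMatchResult removes losers, destroying their pawns, and requeues winners, starting another round once the first list empties.
; An odd player gets a bye.
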(event Custom|Create%20Matches
  (params (IsFirstMatch :type Boolean))
  (if IsFirstMatch
    (Variables|Users|SetSecondPlayerList (Variables|Users|GetPlayerList)))
  (bind _output_get (Variables|Default|SetMatch%20Count (CallFunction|MatchCount)))
  (for _index (range 0 (- _output_get 1))
    (Variables|Default|SetIndex (CallFunction|RandomIndex))
    (while (Utilities|Array|ContainsItem (Variables|Users|GetFIrstPlayerList) (Utilities|Array|Get(acopy) (Variables|Users|GetSecondPlayerList) (Variables|Default|GetIndex)))
      (Variables|Default|SetIndex (CallFunction|RandomIndex)))
    (Utilities|Array|Add (Variables|Users|GetFIrstPlayerList) (Utilities|Array|Get(acopy) (Variables|Users|GetSecondPlayerList) (Variables|Default|GetIndex)))
    (Utilities|Array|RemoveItem (Variables|Users|GetSecondPlayerList) (Utilities|Array|Get(acopy) (Variables|Users|GetSecondPlayerList) (Variables|Default|GetIndex))))
  (CallFunction|GenerateArenas)
  (Utilities|FlowControl|Delay 0.2)
  (CallFunction|StartMatches))

(event Custom|Spawn%20On%20Spawn%20Point
  (params (Player%20Controller :type Player%20Controller%20Object%20Reference) (Location :type Vector) (Rotation :type Rotator))
  (bind _asbp_tournament_player_controller (Utilities|Casting|CastToBP_Tournament_PlayerController Player%20Controller))
  (Transformation|SetActorLocationAndRotation (Pawn|GetControlledPawn _asbp_tournament_player_controller) Location Rotation)
  (Default|UpdatePlayerLocation _asbp_tournament_player_controller Location Rotation))

(event Custom|Start%20Matches
  (if (CallFunction|IsOnePlayerLast)
    (CallFunction|PlayerWon true (CallFunction|GetLastPlayer))
    (elif (CallFunction|IsFirstPlayersIsGreater)
      (CallFunction|UpdateMatchResult (Utilities|Array|Get(acopy) (Variables|Users|GetFIrstPlayerList) (Utilities|Array|LastIndex (Variables|Users|GetFIrstPlayerList))))
      (CallFunction|SpawnPlayeronArenas)
      (else
        (CallFunction|SpawnPlayeronArenas)))))

(event Custom|Player%20Won
  (params (IsLastPlayer :type Boolean) (PlayerController :type Player%20Controller%20Object%20Reference))
  (if IsLastPlayer
    (Development|PrintString "Print Log: Player Won" true true "(R=0.000000,G=0.660000,B=1.000000,A=1.000000)" 1e+02)
    (elif (Utilities|Array|IsEmpty (Variables|Users|GetFIrstPlayerList))
      (CallFunction|CreateMatches false))))

(event Custom|Spawn%20Player%20On%20Arenas
  (for (_array_element _array_index) (Variables|Users|GetFIrstPlayerList)
    (Utilities|FlowControl|Sequence
      (:then_0
        (CallFunction|SpawnonSpawnPoint _array_element (.Location (Class|ContinuousArena2|GetSpawnPoint1Params (Utilities|Array|Get(acopy) (Variables|Default|GetContinuousArenas) _array_index))) (.Rotation (Class|ContinuousArena2|GetSpawnPoint1Params (Utilities|Array|Get(acopy) (Variables|Default|GetContinuousArenas) _array_index)))))
      (:then_1
        (CallFunction|SpawnonSpawnPoint (Utilities|Array|Get(acopy) (Variables|Users|GetSecondPlayerList) _array_index) (.Location (Class|ContinuousArena2|GetSpawnPoint2Params (Utilities|Array|Get(acopy) (Variables|Default|GetContinuousArenas) _array_index))) (.Rotation (Class|ContinuousArena2|GetSpawnPoint2Params (Utilities|Array|Get(acopy) (Variables|Default|GetContinuousArenas) _array_index))))))))

(event Custom|Spawn%20Player%20On%20SpawnPoint
  (params (SpawnPoint :type BP%20CPP%20Spawn%20Point%20on%20Arena%20Object%20Reference) (PlayerController :type Player%20Controller%20Object%20Reference))
  (bind _returnvalue (Transformation|GetActorLocation SpawnPoint))
  (bind _returnvalue_2 (Transformation|GetActorRotation SpawnPoint))
  (bind _asbp_tournament_player_controller (Utilities|Casting|CastToBP_Tournament_PlayerController PlayerController))
  (Transformation|SetActorLocationAndRotation (Pawn|GetControlledPawn _asbp_tournament_player_controller) _returnvalue _returnvalue_2)
  (Default|UpdatePlayerLocation _asbp_tournament_player_controller _returnvalue _returnvalue_2))

(event Custom|Call%20Lost
  (params (NewParam :type Player%20Controller%20Object%20Reference))
  (bind _asbp_tournament_player_controller (Utilities|Casting|CastToBP_Tournament_PlayerController NewParam))
  (Actor|DestroyActor (Pawn|GetControlledPawn _asbp_tournament_player_controller))
  (Default|ServerLost _asbp_tournament_player_controller))

(event Custom|Update%20Match%20Result
  (params (PlayerController%20Won :type Player%20Controller%20Object%20Reference))
  (CallFunction|UpdatePlayerMatches PlayerController%20Won)
  (CallFunction|PlayerWon (CallFunction|IsOnePlayerLast) PlayerController%20Won))

(event Custom|Generate%20Arenas
  (for _array_element (Variables|Users|GetPlayerList)
    (bind _asbp_tournament_player_controller (Utilities|Casting|CastToBP_Tournament_PlayerController _array_element))
    (if (CallFunction|IsFirstPlayersIsGreater)
      (Default|ClientGenerateArenas _asbp_tournament_player_controller (- (Variables|Default|GetMatch%20Count) 1))
      (else
        (Default|ClientGenerateArenas _asbp_tournament_player_controller (Variables|Default|GetMatch%20Count)))))
  (bind _outactors (Actor|GetAllActorsOfClass "/Script/PDP_Tasks.ContinuousArena2"))
  (Variables|Default|SetContinuousArenas _outactors))

(event EventPostLogin
  (params (NewPlayer :type Player%20Controller%20Object%20Reference))
  (Utilities|Array|Add (Variables|Users|GetPlayerList) NewPlayer))

(event EventBeginPlay)

(fn ConstructionScript)

(fn MatchCount
  (bind _secondplayerlist (Variables|Users|GetSecondPlayerList))
  (bind _returnvalue (Utilities|Array|Length _secondplayerlist))
  (return (+ (/ _returnvalue 2) (Math|Integer|%(Integer) _returnvalue 2))))

(fn RandomIndex
  (return (Math|Random|RandomInteger (Variables|Default|GetMatch%20Count))))

(fn IsOnePlayerLast
  (return (or (and (== (Utilities|Array|Length (Variables|Users|GetFIrstPlayerList)) 1) (== (Utilities|Array|Length (Variables|Users|GetSecondPlayerList)) 0)) (and (== (Utilities|Array|Length (Variables|Users|GetFIrstPlayerList)) 0) (== (Utilities|Array|Length (Variables|Users|GetSecondPlayerList)) 1)))))

(fn GetLastPlayer
  (if (== (Utilities|Array|Length (Variables|Users|GetFIrstPlayerList)) 1)
    (return (Utilities|Array|Get(acopy) (Variables|Users|GetFIrstPlayerList)))
    (else
      (return (Utilities|Array|Get(acopy) (Variables|Users|GetSecondPlayerList))))))

(fn IsFirstPlayersIsGreater
  (return (> (Utilities|Array|Length (Variables|Users|GetFIrstPlayerList)) (Utilities|Array|Length (Variables|Users|GetSecondPlayerList)))))

(fn UpdatePlayerMatches
  (params (PlayerController%20Won :type Player%20Controller%20Object%20Reference))
  (bind _secondplayerlist (Variables|Users|GetSecondPlayerList))
  (bind _firstplayerlist (Variables|Users|GetFIrstPlayerList))
  (bind _returnvalue (Utilities|Array|FindItem _secondplayerlist PlayerController%20Won))
  (bind _returnvalue_2 (Utilities|Array|FindItem _firstplayerlist PlayerController%20Won))
  (if (!= _returnvalue_2 -1)
    (if (CallFunction|IsFirstPlayersIsGreater)
      _
      (else
        (CallFunction|CallLost (Utilities|Array|Get(acopy) (Variables|Users|GetSecondPlayerList) _returnvalue_2))
        (Utilities|Array|RemoveIndex (Variables|Users|GetSecondPlayerList) _returnvalue_2)))
    (Utilities|Array|Add (Variables|Users|GetSecondPlayerList) PlayerController%20Won)
    (Utilities|Array|RemoveItem (Variables|Users|GetFIrstPlayerList) PlayerController%20Won)
    (else
      (CallFunction|CallLost (Utilities|Array|Get(acopy) (Variables|Users|GetFIrstPlayerList) _returnvalue))
      (Utilities|Array|RemoveIndex (Variables|Users|GetFIrstPlayerList) _returnvalue))))

(fn GetSpawnPointsOfArena
  (params (ArenaIndex :type Integer))
  (bind _arenaslist (Variables|Default|GetArenasList))
  (bind _output (Utilities|Array|Get(acopy) _arenaslist ArenaIndex))
  (bind _outactors (Actor|GetAttachedActors _output true false))
  (bind _asbp_cpp_spawn_point_on_arena (Utilities|Casting|CastToBP_CPP_SpawnPointOnArena (Utilities|Array|Get(acopy) _outactors))
    (:then
      (bind _asbp_cpp_spawn_point_on_arena_2 (Utilities|Casting|CastToBP_CPP_SpawnPointOnArena (Utilities|Array|Get(acopy) _outactors 1))
        (:then
          (return _asbp_cpp_spawn_point_on_arena _asbp_cpp_spawn_point_on_arena_2))
        (:CastFailed
          _)))
    (:CastFailed
      _))
  (Class|AutomationBlueprintFunctionLibrary|AddExpectedLogError "GameMode: Cast Spawn Point Error"))