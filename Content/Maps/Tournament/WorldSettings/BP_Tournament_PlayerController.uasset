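; Player controller for the tournament map that links each player to match creation, arena setup and match results.
; Pressing P on the server asks BP_Tournament_GameMode to create matches, guarded by a DoOnce.
; Events rebuild arenas through BP_ArenaManager for a given match number and reposition the pawn and view.
; Wins are reported to the game mode, losses destroy the pawn, and local BeginPlay restores game-only input.
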(event Custom|Update%20Player%20Location
  (params (Location :type Vector) (Rotation :type Rotator))
  (Pawn|SetControlRotation Rotation)
  (Transformation|SetActorLocationAndRotation (Pawn|GetControlledPawn) Location Rotation))

(event Custom|Server%20Won
  (bind _asbp_tournament_game_mode (Utilities|Casting|CastToBP_Tournament_GameMode (Game|GetGameMode)))
  (Default|PlayerWon _asbp_tournament_game_mode false self))

(event Custom|Server%20Lost
  (bind _returnvalue (Pawn|GetControlledPawn))
  (Utilities|IsValid _returnvalue
    (:Is%20Valid
      (Actor|DestroyActor _returnvalue))))

(event Custom|Client%20Generate%20Arenas
  (params (MatchNumber :type Integer))
  (bind _returnvalue (Actor|GetActorOfClass "/Game/Maps/ArenasTest/Blueprints/BP_ArenaManager.BP_ArenaManager_C"))
  (Class|ArenaManager|DeleteArenas _returnvalue)
  (Class|ArenaManager|GenerateArenas _returnvalue MatchNumber))

(event Custom|Server%20Start%20Match
  (bind _asbp_tournament_game_mode (Utilities|Casting|CastToBP_Tournament_GameMode (Game|GetGameMode)))
  (Default|CreateMatches _asbp_tournament_game_mode true))

(event EventBeginPlay
  (if (Pawn|IsLocalPlayerController)
    (Viewport|RemoveAllWidgets)
    (Input|SetInputModeGameOnly self false)
    (Variables|Default|SetbShowMouseCursor false)))

(event Input|KeyboardEvents|P
  (params (Key :type Key%20Structure :default "None"))
  (:Pressed
    (if (Networking|IsServer)
      (Utilities|FlowControl|DoOnce false
        (:Completed
          (CallFunction|ServerStartMatch))))))

(fn ConstructionScript)