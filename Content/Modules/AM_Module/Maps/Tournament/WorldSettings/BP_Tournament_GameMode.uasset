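; Game mode for a knockout tournament that starts once the expected player count has logged in and runs rounds until one player remains.
; Players are randomly split into two index-paired lists, then player controllers generate arenas and the mode moves each pair's pawns to spawn points.
; Winners return to the pool for the next round, losers' pawns are destroyed, and an odd player gets a bye.
; Logging out mid-match awards the opponent the win.
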(event Custom|Create%20Matches
  (params (IsFirstMatch :type Boolean))
  (if IsFirstMatch
    (Variables|Users|SetSecondPlayerList (Variables|Users|GetAllConnectedPlayers)))
  (bind _output_get (Variables|Default|SetMatch%20Count (CallFunction|MatchCount)))
  (for _index (range 0 (- _output_get 1))
    (Variables|Default|SetIndex (CallFunction|RandomIndex))
    (while (CallFunction|FPLContainsPlayer)
      (Variables|Default|SetIndex (CallFunction|RandomIndex)))
    (CallFunction|AddPlayertoFPL) ; FPL - FirstPlayerList
  )
  (CallFunction|GenerateArenas)
  (Utilities|FlowControl|Delay 0.2)
  (CallFunction|StartMatches))

(event Custom|Spawn%20On%20Spawn%20Point
  (params (Player%20Controller :type Player%20Controller%20Object%20Reference) (Location :type Vector) (Rotation :type Rotator))
  ;[1 1 1] Spawn Player on Arenas Client
  (bind _asbp_tournament_player_controller (Utilities|Casting|CastToBP_Tournament_PlayerController Player%20Controller))
  (Transformation|SetActorLocationAndRotation (Pawn|GetControlledPawn _asbp_tournament_player_controller) Location Rotation)
  (Default|UpdatePlayerLocation _asbp_tournament_player_controller Location Rotation)
  (CallFunction|UpdatePlayerMatchStatus _asbp_tournament_player_controller "NewEnumerator1"))

(event Custom|Start%20Matches
  (if (CallFunction|IsOnePlayerLast)
    (CallFunction|PlayerWon true (CallFunction|GetLastPlayer))
    (elif (CallFunction|IsFirstPlayersIsGreater)
      (CallFunction|UpdateMatchResult (Utilities|Array|Get(acopy) (Variables|Users|GetFIrstPlayerList) (Utilities|Array|LastIndex (Variables|Users|GetFIrstPlayerList))))
      (CallFunction|SpawnPlayeronArenas)
      (else
        (CallFunction|SpawnPlayeronArenas)))))

(event Custom|Player%20Won
  (params (IsLastPlayer :type Boolean) (PlayerController :type Player%20Controller%20Object%20Reference))
  (bind _asbp_tournament_player_controller (Utilities|Casting|CastToBP_Tournament_PlayerController PlayerController))
  (CallFunction|UpdatePlayerMatchStatus _asbp_tournament_player_controller "NewEnumerator2")
  (if IsLastPlayer
    (CallFunction|PrintWinnerName _asbp_tournament_player_controller)
    (elif (Utilities|Array|IsEmpty (Variables|Users|GetFIrstPlayerList))
      (CallFunction|CreateMatches false))))

(event Custom|Spawn%20Player%20On%20Arenas
  ;[1 1 1] Spawn Player on Arenas Server
  (for (_array_element _array_index) (Variables|Users|GetFIrstPlayerList)
    (Utilities|FlowControl|Sequence
      (:then_0
        (CallFunction|SpawnonSpawnPoint _array_element (.SpawnPointLoc1 (CallFunction|GetTwoSpawnPoints _array_index)) (.SpawnPointRot1 (CallFunction|GetTwoSpawnPoints _array_index))))
      (:then_1
        (CallFunction|SpawnonSpawnPoint (Utilities|Array|Get(acopy) (Variables|Users|GetSecondPlayerList) _array_index) (.SpawnPointLoc2 (CallFunction|GetTwoSpawnPoints _array_index)) (.SpawnPointRot2 (CallFunction|GetTwoSpawnPoints _array_index)))))))

(event Custom|Spawn%20Player%20On%20SpawnPoint
  (params (SpawnPoint :type BP%20CPP%20Spawn%20Point%20on%20Arena%20Object%20Reference) (PlayerController :type Player%20Controller%20Object%20Reference))
  (bind _returnvalue (Transformation|GetActorLocation SpawnPoint))
  (bind _returnvalue_2 (Transformation|GetActorRotation SpawnPoint))
  ;[1 1 1] Utils
  (bind _asbp_tournament_player_controller (Utilities|Casting|CastToBP_Tournament_PlayerController PlayerController))
  (Transformation|SetActorLocationAndRotation (Pawn|GetControlledPawn _asbp_tournament_player_controller) _returnvalue _returnvalue_2)
  (Default|UpdatePlayerLocation _asbp_tournament_player_controller _returnvalue _returnvalue_2))

(event Custom|Player%20Lost
  (params (Player%20Controller :type Player%20Controller%20Object%20Reference))
  (bind _asbp_tournament_player_controller (Utilities|Casting|CastToBP_Tournament_PlayerController Player%20Controller))
  (CallFunction|UpdatePlayerMatchStatus _asbp_tournament_player_controller "NewEnumerator3")
  (Utilities|IsValid (Pawn|GetControlledPawn _asbp_tournament_player_controller)
    (:Is%20Valid
      (Actor|DestroyActor (Pawn|GetControlledPawn _asbp_tournament_player_controller)))
    (:Is%20Not%20Valid
      _))
  (Default|ServerLost _asbp_tournament_player_controller))

(event Custom|Update%20Match%20Result
  (params (PlayerController%20Won :type Player%20Controller%20Object%20Reference))
  (CallFunction|UpdatePlayerMatches PlayerController%20Won)
  (CallFunction|PlayerWon (CallFunction|IsOnePlayerLast) PlayerController%20Won))

(event Custom|Generate%20Arenas
  (for _array_element (Variables|Users|GetAllConnectedPlayers)
    (bind _asbp_tournament_player_controller (Utilities|Casting|CastToBP_Tournament_PlayerController _array_element))
    (if (CallFunction|IsFirstPlayersIsGreater)
      (Default|ClientGenerateArenas _asbp_tournament_player_controller (- (Variables|Default|GetMatch%20Count) 1))
      (else
        (Default|ClientGenerateArenas _asbp_tournament_player_controller (Variables|Default|GetMatch%20Count)))))
  (bind _outactors (Actor|GetAllActorsOfClass "/Script/PDP_Tasks.SimpleArena"))
  (Variables|Default|SetArenasList _outactors))

(event Custom|Update%20Player%20Profiles
  (Utilities|Array|Clear (Variables|Users|GetAllPlayerProfiles))
  (for _array_element (Variables|Users|GetAllConnectedPlayers)
    (bind _asbp_tournament_player_controller (Utilities|Casting|CastToBP_Tournament_PlayerController _array_element))
    (Utilities|Array|Add (Variables|Users|GetAllPlayerProfiles) (Variables|/Game/Modules/AM_Module/Maps/Tournament/WorldSettings/BP_Tournament_PlayerController.BP_Tournament_PlayerController_C|GetPlayerProfile _asbp_tournament_player_controller))))

(event EventOnLogout
  (params (ExitingController :type Controller%20Object%20Reference))
  (bind _asbp_tournament_player_controller (Utilities|Casting|CastToBP_Tournament_PlayerController ExitingController))
  (switch Utilities|FlowControl|Switch|SwitchonE_PlayerStatus (Variables|/Game/Modules/AM_Module/Maps/Tournament/WorldSettings/BP_Tournament_PlayerController.BP_Tournament_PlayerController_C|GetPlayerMatchStatus _asbp_tournament_player_controller)
    (:NewEnumerator0
      (CallFunction|RemoveUserfromLists _asbp_tournament_player_controller :!label _label))
    (:NewEnumerator1
      (CallFunction|RemoveUserinMatch _asbp_tournament_player_controller))
    (:NewEnumerator2
      (goto _label))
    (:NewEnumerator3
      (goto _label))))

(event EventPostLogin
  (params (NewPlayer :type Player%20Controller%20Object%20Reference))
  (Utilities|Array|Add (Variables|Users|GetAllConnectedPlayers) NewPlayer)
  (bind _asbp_tournament_player_controller (Utilities|Casting|CastToBP_Tournament_PlayerController NewPlayer))
  (Default|InitialSetup _asbp_tournament_player_controller)
  (Default|CreateinGameUI _asbp_tournament_player_controller)
  (bind _asbp_game_instance (Utilities|Casting|CastToBP_GameInstance (Game|GetGameInstance)))
  (if (== (Variables|/Game/Modules/AM_Module/Frameworks/BP_GameInstance.BP_GameInstance_C|GetCurrentPlayerNumber _asbp_game_instance) (Utilities|Array|Length (Variables|Users|GetAllConnectedPlayers)))
    (CallFunction|CreateMatches true)))

(event EventBeginPlay
  ;[1 1 1] Utils
)

(fn ConstructionScript)

(fn MatchCount
  (bind _secondplayerlist (Variables|Users|GetSecondPlayerList))
  (bind _returnvalue (Utilities|Array|Length _secondplayerlist))
  (return (+ (/ _returnvalue 2) (Math|Integer|%(Integer) _returnvalue 2))))

(fn RandomIndex
  (return (Math|Random|RandomInteger (Variables|Default|GetMatch%20Count))))

(fn IsOnePlayerLast
  (return (or (and (== (Utilities|Array|Length (Variables|Users|GetFIrstPlayerList)) 1) (== (Utilities|Array|Length (Variables|Users|GetSecondPlayerList)) 0)) (and (== (Utilities|Array|Length (Variables|Users|GetFIrstPlayerList)) 0) (== (Utilities|Array|Length (Variables|Users|GetSecondPlayerList)) 1)))))

(fn GetLastPlayer
  (if (== (Utilities|Array|Length (Variables|Users|GetFIrstPlayerList)) 1)
    (return (Utilities|Array|Get(acopy) (Variables|Users|GetFIrstPlayerList)))
    (else
      (return (Utilities|Array|Get(acopy) (Variables|Users|GetSecondPlayerList))))))

(fn IsFirstPlayersIsGreater
  (return (> (Utilities|Array|Length (Variables|Users|GetFIrstPlayerList)) (Utilities|Array|Length (Variables|Users|GetSecondPlayerList)))))

(fn UpdatePlayerMatches
  (params (PlayerController%20Won :type Player%20Controller%20Object%20Reference))
  (bind _secondplayerlist (Variables|Users|GetSecondPlayerList))
  (bind _firstplayerlist (Variables|Users|GetFIrstPlayerList))
  (bind _returnvalue (Utilities|Array|FindItem _secondplayerlist PlayerController%20Won))
  (bind _returnvalue_2 (Utilities|Array|FindItem _firstplayerlist PlayerController%20Won))
  (if (!= _returnvalue_2 -1)
    (if (CallFunction|IsFirstPlayersIsGreater)
      _
      (else
        (CallFunction|PlayerLost (Utilities|Array|Get(acopy) (Variables|Users|GetSecondPlayerList) _returnvalue_2))
        (Utilities|Array|RemoveIndex (Variables|Users|GetSecondPlayerList) _returnvalue_2)))
    (Utilities|Array|Add (Variables|Users|GetSecondPlayerList) PlayerController%20Won)
    (Utilities|Array|RemoveItem (Variables|Users|GetFIrstPlayerList) PlayerController%20Won)
    (return)
    (else
      (CallFunction|PlayerLost (Utilities|Array|Get(acopy) (Variables|Users|GetFIrstPlayerList) _returnvalue))
      (Utilities|Array|RemoveIndex (Variables|Users|GetFIrstPlayerList) _returnvalue)
      (return))))

(fn FPLContainsPlayer
  (return (Utilities|Array|ContainsItem (Variables|Users|GetFIrstPlayerList) (Utilities|Array|Get(acopy) (Variables|Users|GetSecondPlayerList) (Variables|Default|GetIndex)))))

(fn AddPlayertoFPL
  (bind _secondplayerlist (Variables|Users|GetSecondPlayerList))
  (bind _index (Variables|Default|GetIndex))
  (bind _output (Utilities|Array|Get(acopy) _secondplayerlist _index))
  (Utilities|Array|Add (Variables|Users|GetFIrstPlayerList) _output)
  (Utilities|Array|RemoveItem (Variables|Users|GetSecondPlayerList) _output)
  (return))

(fn UpdatePlayerMatchStatus
  (params (PlayerController :type BP%20Tournament%20Player%20Controller%20Object%20Reference) (NewMatchStatus :type E_PlayerStatus%20Enum :default "NewEnumerator0"))
  (Variables|/Game/Modules/AM_Module/Maps/Tournament/WorldSettings/BP_Tournament_PlayerController.BP_Tournament_PlayerController_C|SetPlayerMatchStatus PlayerController NewMatchStatus)
  (Default|UpdatePlayerStatus PlayerController NewMatchStatus)
  (return))

(fn RemoveUserfromLists
  (params (Disconnected%20Player%20Controller :type Player%20Controller%20Object%20Reference%20%28by%20ref%29))
  (Utilities|Array|RemoveItem (Variables|Users|GetAllConnectedPlayers) Disconnected%20Player%20Controller)
  (Utilities|Array|RemoveItem (Variables|Users|GetFIrstPlayerList) 0)
  (Utilities|Array|RemoveItem (Variables|Users|GetSecondPlayerList) 0)
  (return))

(fn RemoveUserinMatch
  (params (Disconnected%20Player%20Controller :type BP%20Tournament%20Player%20Controller%20Object%20Reference))
  (bind _firstplayerlist (Variables|Users|GetFIrstPlayerList))
  (bind _returnvalue (Utilities|Array|FindItem _firstplayerlist Disconnected%20Player%20Controller))
  (if (!= _returnvalue -1)
    (CallFunction|UpdateMatchResult (Utilities|Array|Get(acopy) (Variables|Users|GetSecondPlayerList) _returnvalue))
    (else
      (CallFunction|UpdateMatchResult (Utilities|Array|Get(acopy) (Variables|Users|GetFIrstPlayerList) (Utilities|Array|FindItem (Variables|Users|GetSecondPlayerList) Disconnected%20Player%20Controller)))))
  (CallFunction|RemoveUserfromLists Disconnected%20Player%20Controller)
  (return))

(fn PrintWinnerName
  (params (PlayerController :type BP%20Tournament%20Player%20Controller%20Object%20Reference))
  (Development|PrintString (Utilities|String|Append (Utilities|String|ToString(Text) (Utilities|Struct|BreakS_PlayerProfile (Variables|/Game/Modules/AM_Module/Maps/Tournament/WorldSettings/BP_Tournament_PlayerController.BP_Tournament_PlayerController_C|GetPlayerProfile PlayerController))) " won Tournament") true true "(R=0.000000,G=0.660000,B=1.000000,A=1.000000)" 1e+02))

(fn GetTwoSpawnPoints
  (params (Arena%20Number :type Integer))
  (bind _arenaslist (Variables|Default|GetArenasList))
  (bind _output (Utilities|Array|Get(acopy) _arenaslist Arena%20Number))
  (bind _spawnpointspositions (Variables|/Script/PDP_Tasks.SimpleArena|GetSpawnPointsPositions _output))
  (bind _spawnpointinfos (Utilities|Struct|BreakSpawnPointsPositions _spawnpointspositions))
  (bind _output_2 (Utilities|Array|Get(acopy) _spawnpointinfos 1))
  (bind _output_3 (Utilities|Array|Get(acopy) _spawnpointinfos))
  (bind (_location _rotation) (Utilities|Struct|BreakSpawnPointInfo _output_2))
  (bind (_location_2 _rotation_2) (Utilities|Struct|BreakSpawnPointInfo _output_3))
  (return _location_2 _rotation_2 _location _rotation))