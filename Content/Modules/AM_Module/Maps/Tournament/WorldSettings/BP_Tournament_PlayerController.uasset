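; Player controller for the tournament mode that links each player to BP_Tournament_GameMode for profiles, match start and results.
; It loads or creates a local save profile and sends it to the server, where the host's T key triggers match creation once.
; Client events generate arenas by match number, while others reposition the pawn, track match status, report wins, destroy losing pawns or leave to MainMenu.
; It also creates the in-game and pause widgets.
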(event Custom|Update%20Player%20Location
  (params (Location :type Vector) (Rotation :type Rotator))
  (Pawn|SetControlRotation Rotation)
  (Transformation|SetActorLocationAndRotation (Pawn|GetControlledPawn) Location Rotation))

(event Custom|Server%20Won
  (bind _asbp_tournament_game_mode (Utilities|Casting|CastToBP_Tournament_GameMode (Game|GetGameMode)))
  (Default|PlayerWon _asbp_tournament_game_mode false self))

(event Custom|Server%20Lost
  (bind _returnvalue (Pawn|GetControlledPawn))
  (Utilities|IsValid _returnvalue
    (:Is%20Valid
      (Actor|DestroyActor _returnvalue))))

(event Custom|Client%20Generate%20Arenas
  (params (MatchNumber :type Integer))
  (bind _returnvalue (Actor|GetActorOfClass "/Script/PDP_Tasks.ArenasGenerator"))
  (Utilities|IsValid _returnvalue
    (:Is%20Valid
      (Class|ArenasGenerator|GenerateArenas _returnvalue false MatchNumber))))

(event Custom|Server%20Start%20Match
  (bind _asbp_tournament_game_mode (Utilities|Casting|CastToBP_Tournament_GameMode (Game|GetGameMode)))
  (Default|CreateMatches _asbp_tournament_game_mode true))

(event Custom|Update%20Player%20Status
  (params (NewParam :type E_PlayerStatus%20Enum :default "NewEnumerator0"))
  (Variables|Default|SetPlayerMatchStatus NewParam))

(event Custom|End%20Client%20Session
  (|DestroySession (Game|GetPlayerController 0)
    (:then
      (Game|OpenLevel(byName) "MainMenu"))))

(event Custom|Initial%20Setup
  (CallFunction|LoadSavedProfile)
  (CallFunction|ServerUpdatePlayerProfile (Variables|Default|GetPlayerProfile)))

(event Custom|Server%20Update%20PlayerProfile
  (params (Player%20Profile :type S%20Player%20Profile%20Structure))
  (Variables|Default|SetPlayerProfile Player%20Profile)
  (bind _asbp_tournament_game_mode (Utilities|Casting|CastToBP_Tournament_GameMode (Game|GetGameMode)))
  (Default|UpdatePlayerProfiles _asbp_tournament_game_mode))

(event Custom|Create%20InGame%20UI
  (CallFunction|UIShowinGame))

(event EventBeginPlay
  (if (Pawn|IsLocalPlayerController)
    (Input|SetInputModeGameOnly self false)
    (Variables|Default|SetbShowMouseCursor false)))

(event Input|KeyboardEvents|P
  (params (Key :type Key%20Structure :default "None"))
  (:Pressed
    (CallFunction|UIShowPauseMenu)))

(event Input|KeyboardEvents|T
  (params (Key :type Key%20Structure :default "None"))
  (:Pressed
    (if (Networking|IsServer)
      (Utilities|FlowControl|DoOnce false
        (:Completed
          (CallFunction|ServerStartMatch))))))

(event Input|KeyboardEvents|Escape
  (params (Key :type Key%20Structure :default "None"))
  (:Pressed
    (CallFunction|UIShowPauseMenu)))

(fn ConstructionScript)

(fn LoadSavedProfile
  (bind _returnvalue (SaveGame|DoesSaveGameExist (LocalVariables|GetLocalSlotName)))
  (if _returnvalue
    _
    (else
      (bind _returnvalue_2 (SaveGame|CreateSaveGameObject "/Game/Modules/AM_Module/Frameworks/SG_PlayerProfile.SG_PlayerProfile_C"))
      (SaveGame|SaveGametoSlot _returnvalue_2 (LocalVariables|GetLocalSlotName))))
  (bind _returnvalue_3 (SaveGame|LoadGamefromSlot (LocalVariables|GetLocalSlotName)))
  (bind _assg_player_profile (Utilities|Casting|CastToSG_PlayerProfile _returnvalue_3))
  (Variables|Default|SetPlayerProfile (Variables|/Game/Modules/AM_Module/Frameworks/SG_PlayerProfile.SG_PlayerProfile_C|GetPlayerProfile _assg_player_profile))
  (return))

(fn UIShowPauseMenu
  (Utilities|IsValid (Variables|Widget|GetPauseMenu_W)
    (:Is%20Valid
      _)
    (:Is%20Not%20Valid
      (bind _returnvalue (UserInterface|CreateWidget "/Game/Modules/AM_Module/Maps/Tournament/UI/WBP_PauseMenu.WBP_PauseMenu_C" self))
      (Variables|Widget|SetPauseMenu_W _returnvalue)))
  (UserInterface|Viewport|AddtoViewport (Variables|Widget|GetPauseMenu_W) 0)
  (Input|SetInputModeUIOnly self 0 "DoNotLock" false)
  (Variables|/Script/Engine.PlayerController|SetbShowMouseCursor self true)
  (return))

(fn UIShowinGame
  (Utilities|IsValid (Variables|Widget|GetInGame_W)
    (:Is%20Valid
      _)
    (:Is%20Not%20Valid
      (bind _returnvalue (UserInterface|CreateWidget "/Game/Modules/AM_Module/Maps/Tournament/UI/WBP_InGameUI.WBP_InGameUI_C" self))
      (Variables|Widget|SetInGame_W _returnvalue)))
  (UserInterface|Viewport|AddtoViewport (Variables|Widget|GetInGame_W) 0)
  (return))